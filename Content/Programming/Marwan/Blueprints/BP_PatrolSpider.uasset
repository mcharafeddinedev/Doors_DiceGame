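; BP_PatrolSpider is a patrolling enemy that kills the player on contact and can be squashed.
; It walks forward every tick and flips 180 degrees when its wall detector begins an overlap or its ledge detector ends one.
; Player detector overlap stops player movement, plays a sound, then after a short delay pauses the game and shows the death widget.
; Squash detector overlap by the player plays a sound and destroys the spider.
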(event `self.ReceiveTick`
  (params (DeltaSeconds :type "Float (single-precision)"))
  (`self.AddMovementInput` (`self.GetActorForwardVector`)))

(event `self.WallDetector.OnComponentBeginOverlap`
  (params (OverlappedComponent :type "PrimitiveComponent Object Reference") (OtherActor :type "Actor Object Reference") (OtherComp :type "PrimitiveComponent Object Reference") (OtherBodyIndex :type Integer) (bFromSweep :type Boolean) (SweepResult :type "HitResult Structure (by ref)"))
  (`self.TurnChar`))

(event `self.LedgeDetector.OnComponentEndOverlap`
  (params (OverlappedComponent :type "PrimitiveComponent Object Reference") (OtherActor :type "Actor Object Reference") (OtherComp :type "PrimitiveComponent Object Reference") (OtherBodyIndex :type Integer))
  (`self.TurnChar`))

(event `self.PlayerDetector.OnComponentBeginOverlap`
  (params (OverlappedComponent :type "PrimitiveComponent Object Reference") (OtherActor :type "Actor Object Reference") (OtherComp :type "PrimitiveComponent Object Reference") (OtherBodyIndex :type Integer) (bFromSweep :type Boolean) (SweepResult :type "HitResult Structure (by ref)"))
  (bind _asbp_player_character (cast `/Game/Programming/Marwan/Blueprints/BP_PlayerCharacter` OtherActor))
  (`Controller.StopMovement` (`PlayerState.GetPlayerController` (`Pawn.PlayerState` _asbp_player_character)))
  (`GameplayStatics.PlaySound2D` "/Game/Programming/Marwan/SFX/SFX_SplatCrunch.SFX_SplatCrunch" 0.15 1.4 0.0 null null)
  (`KismetSystemLibrary.Delay` 0.5)
  (`self.PlayerDeath`))

(event `self.SquashDetector.OnComponentBeginOverlap`
  (params (OverlappedComponent :type "PrimitiveComponent Object Reference") (OtherActor :type "Actor Object Reference") (OtherComp :type "PrimitiveComponent Object Reference") (OtherBodyIndex :type Integer) (bFromSweep :type Boolean) (SweepResult :type "HitResult Structure (by ref)"))
  (cast `/Game/Programming/Marwan/Blueprints/BP_PlayerCharacter` OtherActor)
  (`GameplayStatics.PlaySound2D` "/Game/Programming/Marwan/SFX/SFX_HiddenSpike.SFX_HiddenSpike" 0.75 1.0 0.4 null null)
  (`self.K2_DestroyActor`))

(event `PlayerDeath`
  (`GameplayStatics.SetGamePaused` true)
  (set `PlayerController.bShowMouseCursor` true (`GameplayStatics.GetPlayerController` 0))
  (bind _returnvalue (`|CreateWidget` "/Game/Programming/Eryn/WB_Death.WB_Death_C"))
  (`UserWidget.AddToViewport` _returnvalue 0))

(fn `TurnChar`
  (`self.K2_SetActorRotation` (`KismetMathLibrary.ComposeRotators` (`self.K2_GetActorRotation`) (struct :`Yaw` 180.0))))

(fn `UserConstructionScript`)