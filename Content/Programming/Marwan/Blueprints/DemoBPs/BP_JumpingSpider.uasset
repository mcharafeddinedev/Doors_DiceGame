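; BP_JumpingSpider is a demo Paper2D spider with a collision box, apparently an unfinished jumping hazard for the player.
; StartJump plays a timeline that applies random X and Z impulses to the sprite and box on every update.
; Nothing live calls StartJump, as its looping timer is disconnected.
; Box overlap only casts to BP_PlayerCharacter, with the splat sound, delay and level reload left unwired.
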(event `self.ReceiveTick`
  (params (DeltaSeconds :type "Float (single-precision)")))

(event `self.ReceiveBeginPlay`)

(event `StartJump`
  ;[0.01562 0.01562 0.01562] jump spider logic
  (bind (_direction _jumpcurve) (`Timeline|JumpingTimeline` :!via `PlayFromStart`)
    (:`Update`
      (`PrimitiveComponent.AddImpulse` (`self.PaperSprite`) (`KismetMathLibrary.MakeVector` (`KismetMathLibrary.RandomFloat`) 0.0 (`KismetMathLibrary.RandomFloat`)) "None" false)
      (`PrimitiveComponent.AddImpulse` (`self.CollisionBox`) (`KismetMathLibrary.MakeVector` (`KismetMathLibrary.RandomFloat`) 0.0 (`KismetMathLibrary.RandomFloat`)) "None" false))))

(event `self.CollisionBox.OnComponentBeginOverlap`
  (params (OverlappedComponent :type "PrimitiveComponent Object Reference") (OtherActor :type "Actor Object Reference") (OtherComp :type "PrimitiveComponent Object Reference") (OtherBodyIndex :type Integer) (bFromSweep :type Boolean) (SweepResult :type "HitResult Structure (by ref)"))
  (cast `/Game/Programming/Marwan/Blueprints/BP_PlayerCharacter` OtherActor))

(fn `UserConstructionScript`)