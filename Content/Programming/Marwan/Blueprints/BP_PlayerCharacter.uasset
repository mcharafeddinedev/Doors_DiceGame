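; Player character Blueprint for a 2D knight that walks along X, jumps and toggles a pause menu.
; Move Right and Jump inputs drive movement, the jump sound and directional Paper2D flipbook swaps, with landing restoring idle.
; Tick uses IsJumping and capsule velocity to choose jump flipbooks or sprite scale, but its left-facing checks, like idle's, test Abs(X) < 0 and never pass.
; Pause creates or removes the menu widget, toggling game pause and cursor.
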(event `self.OnLanded`
  (params (Hit :type "HitResult Structure (by ref)"))
  ;[0 0.902 1] MC - Custom Event Verifying isJumping boolean
  (set `self.isJumping` false)
  (`PaperFlipbookComponent.SetFlipbook` (`self.PaperFlipbook`) "/Game/Programming/Marwan/Flipbooks/FB_KnightIdleRight.FB_KnightIdleRight"))

(event `self.ReceiveTick`
  (params (DeltaSeconds :type "Float (single-precision)"))
  ;[0 0.902 1] MC- On Event Tick--> Check If Player isJumping -- On False, Changing Flipbooks' Scale depending on capsule component's velocity, checking velocity for direction when setting Jump Flipbook when isJumping is True
  (if (`self.isJumping`)
    (bind _returnvalue (`PrimitiveComponent.GetPhysicsLinearVelocity` (`self.CapsuleComponent`) "None"))
    (`|ExecutionSequence`
      (:`then_0`
        (bind _x (.x _returnvalue))
        (if (< (`KismetMathLibrary.Abs` _x) 0.0)
          (`PaperFlipbookComponent.SetFlipbook` (`self.PaperFlipbook`) "/Game/Programming/Marwan/Flipbooks/FB_KnightJumpLeft.FB_KnightJumpLeft")))
      (:`then_1`
        (if (> (`KismetMathLibrary.Abs` _x) 0.0)
          (`PaperFlipbookComponent.SetFlipbook` (`self.PaperFlipbook`) "/Game/Programming/Marwan/Flipbooks/FB_KnightJumpRight.FB_KnightJumpRight"))))
    (else
      (bind _returnvalue_2 (`PrimitiveComponent.GetPhysicsLinearVelocity` (`self.CapsuleComponent`) "None"))
      (`|ExecutionSequence`
        (:`then_0`
          (bind _x_2 (.x _returnvalue_2))
          (if (< (`KismetMathLibrary.Abs` _x_2) 0.0)
            (`SceneComponent.SetRelativeScale3D` (`self.PaperFlipbook`) (-1.0 1.0 1.0))))
        (:`then_1`
          (if (> (`KismetMathLibrary.Abs` _x_2) 0.0)
            (`SceneComponent.SetRelativeScale3D` (`self.PaperFlipbook`) (1.0 1.0 1.0))))))))

(event `InputAction|Pause`
  (params (Key :type "Key Structure"))
  ;[0 0.9804 1] Pause Logic -- M.C.
  (:`Pressed`
    (if (`GameplayStatics.IsGamePaused`)
      (`GameplayStatics.SetGamePaused` false)
      (`Widget.RemoveFromParent` (`self.REF_W_PauseMenuPopup`))
      (set `PlayerController.bShowMouseCursor` false (`GameplayStatics.GetPlayerController` 0))
      (else
        (bind _returnvalue (`|CreateWidget` "/Game/Programming/Marwan/Widgets/W_PauseMenuPopUp.W_PauseMenuPopUp_C"))
        (bind _output_get (set `self.REF_W_PauseMenuPopup` _returnvalue))
        (`UserWidget.AddToViewport` _output_get 0)
        (`GameplayStatics.SetGamePaused` true)
        (set `PlayerController.bShowMouseCursor` true (`GameplayStatics.GetPlayerController` 0))))))

(event `InputAxis|Move Right`
  (params (AxisValue :type "Float (single-precision)"))
  ;[0 0.9804 1] Movement Logic with Sprite Flipbooks -- M.C.
  ;;[1 1 1] MoveRight
  (`self.AddMovementInput` (1.0 0.0 0.0) AxisValue)
  (if (> AxisValue 0.0)
    (`PaperFlipbookComponent.SetFlipbook` (`self.PaperFlipbook`) "/Game/Programming/Marwan/Flipbooks/FB_KnightWalkRight.FB_KnightWalkRight")
    (else
      ;;[1 1 1] Idle
      (if (== AxisValue 0.0)
        (bind _returnvalue (`PrimitiveComponent.GetPhysicsLinearVelocity` (`self.CapsuleComponent`) "None"))
        (`|ExecutionSequence`
          (:`then_0`
            (bind _x (.x _returnvalue))
            (if (< (`KismetMathLibrary.Abs` _x) 0.0)
              (`PaperFlipbookComponent.SetFlipbook` (`self.PaperFlipbook`) "/Game/Programming/Marwan/Flipbooks/FB_KnightIdleLeft.FB_KnightIdleLeft")))
          (:`then_1`
            (if (> (`KismetMathLibrary.Abs` _x) 0.0)
              (`PaperFlipbookComponent.SetFlipbook` (`self.PaperFlipbook`) "/Game/Programming/Marwan/Flipbooks/FB_KnightIdleRight.FB_KnightIdleRight"))))
        (else
          ;;[1 1 1] MoveLeft
          (if (< AxisValue 0.0)
            (`PaperFlipbookComponent.SetFlipbook` (`self.PaperFlipbook`) "/Game/Programming/Marwan/Flipbooks/FB_KnightWalkLeft.FB_KnightWalkLeft")
            (`self.AddMovementInput` (1.0 0.0 0.0) AxisValue)))))))

(event `InputAction|Jump`
  (params (Key :type "Key Structure"))
  ;[0 0.9804 1] Movement Logic with Sprite Flipbooks -- M.C.
  ;;[0 0.902 1] Jump Logic -- M.C.
  (:`Pressed`
    (set `self.isJumping` true)
    (`PaperFlipbookComponent.SetFlipbook` (`self.PaperFlipbook`) "/Game/Programming/Marwan/Flipbooks/FB_KnightJumpRight.FB_KnightJumpRight")
    (`self.Jump`)
    (`GameplayStatics.PlaySound2D` "/Game/Programming/Marwan/SFX/SC_JumpSounds.SC_JumpSounds" 1.0 1.0 0.0 null null))
  (:`Released`
    (`self.StopJumping`)
    (set `self.isJumping` false)
    (`PaperFlipbookComponent.SetFlipbook` (`self.PaperFlipbook`) "/Game/Programming/Marwan/Flipbooks/FB_KnightIdleRight.FB_KnightIdleRight")))

(fn `UserConstructionScript`)